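; Player character Blueprint for camera-relative movement, with controller look input and a jump-button flag.
; Tick feeds VelocityVector into movement input, rebuilding it from camera vectors and move axes, or keeping the last one when the axes sum to zero.
; A gate opened by Predict or UsePlayerRotation eases yaw toward that vector until movement stops or UseCharacterRotation closes it.
; CalculateStartAnimation maps the actor-to-vector yaw difference to a directional stand-to-jog animation.
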(event Custom|UsePlayerRotation
  (Utilities|FlowControl|Gate true) ; enters at Open
)

(event Custom|Predict
  (CallFunction|UsePlayerRotation))

(event Custom|UseCharacterRotation
  (Utilities|FlowControl|Gate true) ; enters at Close
)

(event EventBeginPlay)

(event Collision|EventActorBeginOverlap
  (params (OtherActor :type Actor%20Object%20Reference)))

(event EventTick
  (params (DeltaSeconds :type Float%20%28single-precision%29))
  (Pawn|Input|AddMovementInput (Variables|Default|GetVelocityVector) 1.0 false)
  (|SetVelocityVector)
  (Utilities|FlowControl|Sequence
    (:then_0
      (Utilities|FlowControl|Gate true :!label _label
        (:Exit
          (Transformation|SetActorRotation (Math|Rotator|MakeRotator 0.0 0.0 (.yaw (Math|Interpolation|RInterpTo (Transformation|GetActorRotation) (Math|Rotator|MakeRotfromX (Variables|Default|GetVelocityVector)) (Utilities|Time|GetWorldDeltaSeconds) 6.0)))))))
    (:then_1
      (bind _output_get (Variables|Default|SetIsMoving (not (== (+ (Math|Float|Absolute(Float) (Input|AxisValues|GetMoveForward)) (Math|Float|Absolute(Float) (Input|AxisValues|GetMoveRight))) 0.0))))
      (if (not _output_get)
        (goto _label Close)))))

(event EventOnLanded
  (params (Hit :type Hit%20Result%20Structure%20%28by%20ref%29))
  (Variables|Default|SetjumpButtonDown? false))

(event Input|ActionEvents|InputActionJump
  (params (Key :type Key%20Structure))
  (:Pressed
    (Variables|Default|SetjumpButtonDown? true))
  (:Released
    (if (not (Variables|Default|GetIsMoving))
      (Variables|Default|SetjumpButtonDown? false))))

(event Input|AxisEvents|InputAxisTurn
  (params (AxisValue :type Float%20%28single-precision%29))
  (Pawn|Input|AddControllerPitchInput AxisValue))

(event Input|AxisEvents|InputAxisLookUpRate
  (params (AxisValue :type Float%20%28single-precision%29))
  (Pawn|Input|AddControllerPitchInput (* AxisValue (Variables|Default|GetControllerSensitivity) (Utilities|Time|GetWorldDeltaSeconds))))

(event Input|AxisEvents|InputAxisTurnRate
  (params (AxisValue :type Float%20%28single-precision%29))
  (Pawn|Input|AddControllerYawInput (* AxisValue (Variables|Default|GetControllerSensitivity) (Utilities|Time|GetWorldDeltaSeconds))))

(event Input|AxisEvents|InputAxisLookUp
  (params (AxisValue :type Float%20%28single-precision%29))
  (Pawn|Input|AddControllerYawInput AxisValue))

(fn ConstructionScript)

(fn GetVectors
  (bind _camera (Variables|Default|GetCamera))
  (return (Math|Vector|GetForwardVector _camera) (Math|Vector|GetRightVector _camera)))

(fn CalculateStartAnimation
  (bind _returnvalue (Transformation|GetActorRotation))
  (bind _velocityvector (Variables|Default|GetVelocityVector))
  (bind _returnvalue_2 (Math|Rotator|MakeRotfromX _velocityvector))
  (bind _returnvalue_3 (Math|Rotator|Delta(Rotator) _returnvalue _returnvalue_2))
  (if (Math|Float|InRange(Float) (.yaw _returnvalue_3) -2e+01 2e+01)
    (LocalVariables|SetDesiredAnimAsset "/Game/TransferDump/ControllerMain/Animations/InPlace/MOB1_Stand_Relaxed_to_Jog_F_IPC.MOB1_Stand_Relaxed_to_Jog_F_IPC")
    (elif (Math|Float|InRange(Float) (.yaw _returnvalue_3) -6e+01 -21.0)
      (LocalVariables|SetDesiredAnimAsset "/Game/TransferDump/ControllerMain/Animations/InPlace/MOB1_Stand_Relaxed_To_Jog_R45_Fwd_IPC.MOB1_Stand_Relaxed_To_Jog_R45_Fwd_IPC")
      (elif (Math|Float|InRange(Float) (.yaw _returnvalue_3) -1.1e+02 -61.0)
        (LocalVariables|SetDesiredAnimAsset "/Game/TransferDump/ControllerMain/Animations/InPlace/MOB1_Stand_Relaxed_To_Jog_R90_Fwd_IPC.MOB1_Stand_Relaxed_To_Jog_R90_Fwd_IPC")
        (elif (Math|Float|InRange(Float) (.yaw _returnvalue_3) -155.0 -1.1e+02)
          (LocalVariables|SetDesiredAnimAsset "/Game/TransferDump/ControllerMain/Animations/InPlace/MOB1_Stand_Relaxed_To_Jog_R135_Fwd_IPC.MOB1_Stand_Relaxed_To_Jog_R135_Fwd_IPC")
          (elif (Math|Float|InRange(Float) (.yaw _returnvalue_3) -1.8e+02 -155.0)
            (LocalVariables|SetDesiredAnimAsset "/Game/TransferDump/ControllerMain/Animations/InPlace/MOB1_Stand_Relaxed_To_Jog_R180_Fwd_IPC.MOB1_Stand_Relaxed_To_Jog_R180_Fwd_IPC")
            (elif (Math|Float|InRange(Float) (.yaw _returnvalue_3) 2e+01 6e+01)
              (LocalVariables|SetDesiredAnimAsset "/Game/TransferDump/ControllerMain/Animations/InPlace/MOB1_Stand_Relaxed_To_Jog_L45_Fwd_IPC.MOB1_Stand_Relaxed_To_Jog_L45_Fwd_IPC")
              (elif (Math|Float|InRange(Float) (.yaw _returnvalue_3) 6e+01 1.1e+02)
                (LocalVariables|SetDesiredAnimAsset "/Game/TransferDump/ControllerMain/Animations/InPlace/MOB1_Stand_Relaxed_To_Jog_L90_Fwd_IPC.MOB1_Stand_Relaxed_To_Jog_L90_Fwd_IPC")
                (elif (Math|Float|InRange(Float) (.yaw _returnvalue_3) 1.1e+02 155.0)
                  (LocalVariables|SetDesiredAnimAsset "/Game/TransferDump/ControllerMain/Animations/InPlace/MOB1_Stand_Relaxed_To_Jog_L135_Fwd_IPC.MOB1_Stand_Relaxed_To_Jog_L135_Fwd_IPC")
                  (elif (Math|Float|InRange(Float) (.yaw _returnvalue_3) 155.0 1.8e+02)
                    (LocalVariables|SetDesiredAnimAsset "/Game/TransferDump/ControllerMain/Animations/InPlace/MOB1_Stand_Relaxed_To_Jog_L180_Fwd_IPC.MOB1_Stand_Relaxed_To_Jog_L180_Fwd_IPC"))))))))))
  (return (LocalVariables|GetDesiredAnimAsset)))