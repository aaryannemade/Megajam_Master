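; Light_Platform is a puzzle element that moves a referenced MovingActor between two positions marked by its Pos1 and Pos2 components.
; On BeginPlay it snaps the actor, if valid, to the position selected by the IsInPos1 flag.
; SwitchPosition flips that flag and restarts the TransitionSpeed timeline, which lerps the actor from the previous position to the new one without sweeping.
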(event Custom|SwitchPosition
  (if (Variables|Default|GetIsInPos1?)
    (Variables|Default|SetIsInPos1? false)
    (bind _alpha (Timeline|Transition%20Speed PlayFromStart)
      (:Update
        (Transformation|SetActorLocation (Variables|Default|GetMovingActor) (Math|Vector|Lerp(Vector) (Math|Vector|SelectVector (Transformation|GetWorldLocation (Variables|Default|GetPos2)) (Transformation|GetWorldLocation (Variables|Default|GetPos1)) (Variables|Default|GetIsInPos1?)) (Math|Vector|SelectVector (Transformation|GetWorldLocation (Variables|Default|GetPos1)) (Transformation|GetWorldLocation (Variables|Default|GetPos2)) (Variables|Default|GetIsInPos1?)) _alpha) false false)))
    (else
      (Variables|Default|SetIsInPos1? true)
      (Timeline|Transition%20Speed PlayFromStart))))

(event EventBeginPlay
  (Utilities|IsValid (Variables|Default|GetMovingActor)
    (:Is%20Valid
      (Transformation|SetActorLocation (Variables|Default|GetMovingActor) (Math|Vector|SelectVector (Transformation|GetWorldLocation (Variables|Default|GetPos1)) (Transformation|GetWorldLocation (Variables|Default|GetPos2)) (Variables|Default|GetIsInPos1?)) false false))))

(fn ConstructionScript)