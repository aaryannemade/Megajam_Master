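; LightCube is a puzzle element that lights its point light when activated and can pass that activation on to a linked Emitter.
; ActivateLight raises the light intensity, sets the active flag and, if enabled, activates the Emitter.
; While active and linked, Tick checks the distance between both cubes against a maximum to switch the Emitter on or off.
; Two cross-resetting DoOnce gates limit those calls to range changes.
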(event Custom|ActivateLight
  (bind _emitter (Variables|Default|GetEmitter))
  (Rendering|Components|Light|SetIntensity (Variables|Default|GetPointLight) 5e+03)
  (Variables|Default|SetIsLightActive true)
  (if (Variables|Default|GetActivateEmitter?)
    (Utilities|IsValid _emitter
      (:Is%20Valid
        (Default|ActivateLight _emitter)))))

(event EventBeginPlay)

(event Collision|EventActorBeginOverlap
  (params (OtherActor :type Actor%20Object%20Reference)))

(event EventTick
  (params (DeltaSeconds :type Float%20%28single-precision%29))
  (bind _emitter (Variables|Default|GetEmitter))
  (if (and (Variables|Default|GetActivateEmitter?) (Variables|Default|GetIsLightActive))
    (if (< (Math|Vector|VectorLength (- (Transformation|GetWorldLocation (Variables|Default|GetCube)) (Transformation|GetWorldLocation (Variables|/Game/Blueprints/PuzzleElements/LightEmitter.LightEmitter_C|GetCube (Variables|Default|GetEmitter))))) (Variables|Default|GetMaximumDistance))
      (Utilities|FlowControl|DoOnce false :!label _label
        (:Completed
          (Default|ActivateLight _emitter)
          (goto _label_2 Reset)))
      (else
        (Utilities|FlowControl|DoOnce false :!label _label_2
          (:Completed
            (Default|DeactivateLight _emitter)
            (goto _label Reset)))))))

(fn ConstructionScript)