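; LightEmitter is a puzzle element that passes a light signal along a chain of emitters.
; Once activated, a looping timer debug-traces along the emit location's up vector, setting itself as the source of any new emitter hit.
; Relayed emitters poll that their source still hits them, otherwise deactivating and cascading the shutdown downstream.
; Auto light sources skip that check and ignore deactivation.
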(event Custom|TraceLight
  (bind _emitlocation (Variables|Default|GetEmitLocation))
  (bind _returnvalue (Transformation|GetWorldLocation _emitlocation))
  (bind (_outhit _returnvalue_2) (Collision|LineTraceByChannel _returnvalue (+ _returnvalue (* (Math|Vector|GetUpVector _emitlocation) 5e+02)) "TraceTypeQuery1" false 0 "ForDuration"))
  (if _returnvalue_2
    (Utilities|IsValid (.HitActor (Collision|BreakHitResult _outhit))
      (:Is%20Valid
        (if (not (== (.HitActor (Collision|BreakHitResult _outhit)) (Variables|Default|GetHitActor)))
          (bind _aslight_emitter (Utilities|Casting|CastToLightEmitter (.HitActor (Collision|BreakHitResult _outhit))))
          (bind _output_get (Variables|Default|SetHitActor _aslight_emitter))
          (CallFunction|SetSource _output_get self))))
    (else
      (Utilities|IsValid (Variables|Default|GetHitActor)
        (:Is%20Valid
          (CallFunction|DeactivateLight (Variables|Default|GetHitActor))
          (Variables|Default|SetHitActor 0))))))

(event Custom|DeactivateLight
  (bind _hitactor (Variables|Default|GetHitActor))
  (if (not (Variables|Default|GetAutoLightSource?))
    (Variables|Default|SetHasLightSource false)
    (Utilities|Time|ClearTimerbyFunctionName 0 "CheckLightSource")
    (Utilities|Time|ClearTimerbyFunctionName 0 "TraceLight")
    (Variables|Default|SetLightActivated false)
    (Utilities|IsValid _hitactor
      (:Is%20Valid
        (CallFunction|DeactivateLight _hitactor)))))

(event Custom|ActivateLight
  (if (Variables|Default|GetAutoLightSource?)
    (Utilities|Time|SetTimerbyFunctionName 0 "TraceLight" 1.0 true)
    (Variables|Default|SetLightActivated true)
    (else
      (Utilities|Time|SetTimerbyFunctionName 0 "CheckLightSource" 1.0 true)
      (Utilities|Time|SetTimerbyFunctionName 0 "TraceLight" 1.0 true)
      (Variables|Default|SetLightActivated true))))

(event Custom|SetSource
  (params (Source :type Light%20Emitter%20Object%20Reference))
  (Variables|Default|SetSource Source)
  (CallFunction|ActivateLight))

(event Custom|CheckLightSource
  (bind _source (Variables|Default|GetSource))
  (Utilities|IsValid _source
    (:Is%20Valid
      (bind _output_get (Variables|Default|SetHasLightSource (== (Variables|LightEmitter_C|GetHitActor _source) self)))
      (if (not _output_get)
        (CallFunction|DeactivateLight :!label _label)))
    (:Is%20Not%20Valid
      (Variables|Default|SetHasLightSource false)
      (goto _label))))

(event EventBeginPlay)

(event Collision|EventActorBeginOverlap
  (params (OtherActor :type Actor%20Object%20Reference)))

(event EventTick
  (params (DeltaSeconds :type Float%20%28single-precision%29)))

(fn ConstructionScript)