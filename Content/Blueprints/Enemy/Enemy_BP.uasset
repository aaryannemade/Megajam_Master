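; Enemy pawn that wanders the navmesh, chases the player on sight and lowers the player's light bar when close.
; FindNewLocation loops random AIMoveTo wandering, fading out chase music after a successful move.
; PawnSensing speeds up pursuit, while a DoOnce gates the player notification, alert sound and delayed chase music.
; The Teleported event slows the enemy, restarts wandering and re-arms that alert.
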(event OnSeePawn(PawnSensing)
  (params (Pawn :type Pawn%20Object%20Reference))
  (bind _asplayer_bp (Utilities|Casting|CastToPlayer_BP Pawn))
  (Utilities|FlowControl|Sequence
    (:then_0
      (Components|Movement|StopMovementImmediately (Variables|Character|GetCharacterMovement))
      (Variables|/Script/Engine.CharacterMovementComponent|SetMaxWalkSpeed (Variables|Character|GetCharacterMovement) 4e+02)
      (AI|AIMoveTo self "0, 0, 0" (Variables|Default|GetPlayerCharacter) 5.0 false))
    (:then_1
      (Utilities|FlowControl|DoOnce false
        (:Completed
          (Default|EnemyChasing _asplayer_bp self)
          (Audio|PlaySound2D "/Game/Sounds/SFX_EnemyAlert.SFX_EnemyAlert")
          (Variables|Default|SetIsFollowing true)
          (Utilities|FlowControl|Delay 4.0)
          (if (Variables|Default|GetIsFollowing)
            _
            (else
              _))
          (bind _returnvalue (Audio|SpawnSound2D "/Game/Sounds/Music_Chase_Loop.Music_Chase_Loop"))
          (Variables|Default|SetChaseSound _returnvalue))))))

(event Custom|FindNewLocation
  (bind _returnvalue (Transformation|GetActorLocation))
  (bind _chasesound (Variables|Default|GetChaseSound))
  (bind (_randomlocation _returnvalue_2) (Class|NavigationSystem|GetRandomPointinNavigableRadius _returnvalue 5e+02))
  (Variables|Default|SetIsFollowing false)
  (AI|AIMoveTo self (Math|Vector|SelectVector _randomlocation "0, 0, 0" _returnvalue_2) 0 5.0 false
    (:OnSuccess
      (Utilities|FlowControl|Delay 1.0)
      (CallFunction|FindNewLocation)
      (Utilities|IsValid _chasesound
        (:Is%20Valid
          (Audio|Components|Audio|FadeOut _chasesound 2.0 0.0 :!class /Script/Engine.AudioComponent)
          (Audio|Components|Audio|Stop _chasesound))))))

(event Custom|Teleported
  (Components|Movement|StopMovementImmediately (Variables|Character|GetCharacterMovement))
  (Variables|/Script/Engine.CharacterMovementComponent|SetMaxWalkSpeed (Variables|Character|GetCharacterMovement) 1e+02)
  (CallFunction|FindNewLocation)
  (Utilities|FlowControl|DoOnce false) ; enters at Reset
)

(event EventBeginPlay
  (bind _asplayer_bp (Utilities|Casting|CastToPlayer_BP (Game|GetPlayerCharacter 0)))
  (Variables|Default|SetPlayerCharacter _asplayer_bp)
  (Utilities|FlowControl|Delay 2.0)
  (CallFunction|FindNewLocation))

(event Collision|EventActorBeginOverlap
  (params (OtherActor :type Actor%20Object%20Reference)))

(event EventTick
  (params (DeltaSeconds :type Float%20%28single-precision%29))
  (if (< (Math|Vector|VectorLength (- (Transformation|GetWorldLocation (Variables|/Script/Engine.Character|GetMesh (Variables|Default|GetPlayerCharacter))) (Transformation|GetActorLocation))) 2e+02)
    (Utilities|FlowControl|Delay 2.0)
    (Default|LowerLightBar (Variables|Default|GetPlayerCharacter))))

(fn ConstructionScript)