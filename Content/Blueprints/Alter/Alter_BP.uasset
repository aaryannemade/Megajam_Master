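; Alter_BP is an altar-style actor with a pyramid mesh and text that react to the player's proximity.
; Each Tick it maps the player's distance to the pyramid's Emissive material parameter, so the glow grows as the player approaches and fades out at range.
; Overlaps on a trigger component show the text render when Player_BP enters and hide it when Player_BP leaves.
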(event OnComponentBeginOverlap(TextVisisbilityCollision)
  (params (OverlappedComponent :type Primitive%20Component%20Object%20Reference) (OtherActor :type Actor%20Object%20Reference) (OtherComp :type Primitive%20Component%20Object%20Reference) (OtherBodyIndex :type Integer) (bFromSweep :type Boolean) (SweepResult :type Hit%20Result%20Structure%20%28by%20ref%29))
  (Utilities|Casting|CastToPlayer_BP OtherActor)
  (Development|SetHiddeninGame (Variables|Default|GetTextRender) false false))

(event OnComponentEndOverlap(TextVisisbilityCollision)
  (params (OverlappedComponent :type Primitive%20Component%20Object%20Reference) (OtherActor :type Actor%20Object%20Reference) (OtherComp :type Primitive%20Component%20Object%20Reference) (OtherBodyIndex :type Integer))
  (Utilities|Casting|CastToPlayer_BP OtherActor)
  (Development|SetHiddeninGame (Variables|Default|GetTextRender) true false))

(event EventBeginPlay)

(event Collision|EventActorBeginOverlap
  (params (OtherActor :type Actor%20Object%20Reference)))

(event EventTick
  (params (DeltaSeconds :type Float%20%28single-precision%29))
  (Rendering|Material|SetScalarParameterValueonMaterials (Variables|Default|GetPyramid) "Emissive" (Math|Float|MapRangeClamped (Math|Vector|VectorLength (- (Transformation|GetActorLocation) (Transformation|GetWorldLocation (Variables|/Script/Engine.Character|GetCapsuleComponent (Game|GetPlayerCharacter 0))))) 1.5e+03 5e+03 6.0 0.0)))

(fn ConstructionScript)