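; Player character with camera-relative movement, a draining light bar and a light projectile aimed by camera trace.
; Tick turns the body toward the last input direction at a speed-scaled rate and triggers the AnimBP start animation, with CalculateStartAnimation choosing directional jog starts by yaw delta.
; A looping timeline drains light; at exactly zero, the player leaves a Silhouette posed from the mesh's socket transforms and teleports back to the starting location.
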(event Custom|Initialise%20LightBar
  (Variables|Default|SetLightBarValue (Variables|Default|GetLightBarMaxValue))
  (CallFunction|StartLightBar))

(event Custom|StartLightBar
  (Timeline|LightBar Play
    (:Loop%20every%201%20second
      (bind _output_get (Variables|Default|SetLightBarValue (- (Variables|Default|GetLightBarValue) (* (Variables|Default|GetDechargeRate) 10))))
      (if (== _output_get 0)
        (CallFunction|RespawnCharacter)))))

(event Custom|SpawnSilhouette
  (for _array_element (Transformation|GetAllSocketNames (Variables|Character|GetMesh))
    (Utilities|Array|Add (Variables|Default|GetBoneLocations) (Transformation|GetSocketTransform (Variables|Character|GetMesh) _array_element "RTS_World")))
  (bind _returnvalue (Game|SpawnActorfromClass "/Game/Blueprints/Player/Silhouette.Silhouette_C" (Transformation|GetActorTransform) "AlwaysSpawn" 0 0))
  (Default|SetBoneTransform _returnvalue (Variables|Default|GetBoneLocations))
  (Utilities|Array|Clear (Variables|Default|GetBoneLocations)))

(event Custom|StopLightBar
  (Timeline|LightBar Stop
    (:Loop%20every%201%20second
      (bind _output_get (Variables|Default|SetLightBarValue (- (Variables|Default|GetLightBarValue) (* (Variables|Default|GetDechargeRate) 10))))
      (if (== _output_get 0)
        (CallFunction|RespawnCharacter)))))

(event Custom|RespawnCharacter
  (bind _startinglocation (Variables|Default|GetStartingLocation))
  (bind (_location _rotation) (Math|Transform|BreakTransform _startinglocation))
  (CallFunction|StopLightBar)
  (CallFunction|InitialiseLightBar)
  (CallFunction|SpawnSilhouette)
  (Transformation|Teleport _location _rotation))

(event EventBeginPlay
  (bind _asplayer_anim_bp (Utilities|Casting|CastToPlayerAnimBP (Components|SkeletalMesh|GetAnimInstance (Variables|Character|GetMesh))))
  (Variables|Default|SetAnimBP _asplayer_anim_bp)
  (CallFunction|InitialiseLightBar)
  (Variables|Default|SetStartingLocation (Transformation|GetActorTransform)))

(event Collision|EventActorBeginOverlap
  (params (OtherActor :type Actor%20Object%20Reference)))

(event EventTick
  (params (DeltaSeconds :type Float%20%28single-precision%29))
  (Pawn|Input|AddMovementInput (Variables|Default|GetVelocityVector) 1.0 false)
  (|SetVelocityVector)
  (Utilities|FlowControl|Sequence
    (:then_0
      (Utilities|FlowControl|Sequence
        (:then_0
          (Development|PrintString (Utilities|String|ToString(Integer) (Variables|Default|GetLightBarValue)) true true "(R=0.000000,G=0.660000,B=1.000000,A=1.000000)" (Utilities|Time|GetWorldDeltaSeconds)))))
    (:then_1
      (Transformation|SetActorRotation (Math|Rotator|MakeRotator 0.0 0.0 (.yaw (Math|Interpolation|RInterpTo (Transformation|GetActorRotation) (Math|Rotator|MakeRotfromX (Variables|Default|GetVelocityVector)) (Utilities|Time|GetWorldDeltaSeconds) (Math|Float|MapRangeClamped (Math|Vector|VectorLength (Transformation|GetVelocity)) 1e+02 346.0 1.0 5.0))))))
    (:then_2
      (bind _output_get (Variables|Default|SetIsMoving (not (== (+ (Math|Float|Absolute(Float) (Input|AxisValues|GetMoveForward)) (Math|Float|Absolute(Float) (Input|AxisValues|GetMoveRight))) 0.0))))
      (if _output_get
        (Utilities|FlowControl|DoOnce true :!label _label
          (:Completed
            (Default|StartAnim (Variables|Default|GetAnimBP))))
        (else
          (goto _label Reset))))))

(event EventOnLanded
  (params (Hit :type Hit%20Result%20Structure%20%28by%20ref%29))
  (Variables|Default|SetjumpButtonDown? false))

(event Input|ActionEvents|InputActionJump
  (params (Key :type Key%20Structure))
  (:Pressed
    (Variables|Default|SetjumpButtonDown? true))
  (:Released
    (if (not (Variables|Default|GetIsMoving))
      (Variables|Default|SetjumpButtonDown? false))))

(event Input|ActionEvents|InputActionProjectile
  (params (Key :type Key%20Structure))
  (bind _capsulecomponent (Variables|Collision|GetCapsuleComponent))
  (bind _camera (Variables|Default|GetCamera))
  (bind _returnvalue (Transformation|GetWorldLocation _camera))
  (bind _returnvalue_2 (Transformation|GetWorldLocation _capsulecomponent))
  (:Pressed
    (bind (_outhit _returnvalue_3) (Collision|LineTraceByChannel _returnvalue (+ _returnvalue (* (Math|Vector|GetForwardVector _camera) 99999.0)) "TraceTypeQuery1" false 0 "ForDuration"))
    (if _returnvalue_3
      (Game|SpawnActorfromClass "/Game/Blueprints/Player/Projectile/LightProjectile.LightProjectile_C" (Math|Transform|MakeTransform _returnvalue_2 (Math|Rotator|FindLookatRotation _returnvalue_2 (.Location (Collision|BreakHitResult _outhit)))) "AlwaysSpawn" 0 0)
      (else
        (Game|SpawnActorfromClass "/Game/Blueprints/Player/Projectile/LightProjectile.LightProjectile_C" (Math|Transform|MakeTransform _returnvalue_2 (Math|Rotator|FindLookatRotation _returnvalue_2 (.TraceEnd (Collision|BreakHitResult _outhit)))) "AlwaysSpawn" 0 0)))))

(event Input|AxisEvents|InputAxisTurn
  (params (AxisValue :type Float%20%28single-precision%29))
  (Pawn|Input|AddControllerYawInput AxisValue))

(event Input|AxisEvents|InputAxisLookUpRate
  (params (AxisValue :type Float%20%28single-precision%29))
  (Pawn|Input|AddControllerPitchInput (* AxisValue (Variables|Default|GetControllerSensitivity) (Utilities|Time|GetWorldDeltaSeconds))))

(event Input|AxisEvents|InputAxisTurnRate
  (params (AxisValue :type Float%20%28single-precision%29))
  (Pawn|Input|AddControllerYawInput (* AxisValue (Variables|Default|GetControllerSensitivity) (Utilities|Time|GetWorldDeltaSeconds))))

(event Input|AxisEvents|InputAxisLookUp
  (params (AxisValue :type Float%20%28single-precision%29))
  (Pawn|Input|AddControllerPitchInput AxisValue))

(fn ConstructionScript)

(fn GetVectors
  (bind _camera (Variables|Default|GetCamera))
  (return (Math|Vector|GetForwardVector _camera) (Math|Vector|GetRightVector _camera)))

(fn CalculateStartAnimation
  (bind _returnvalue (Transformation|GetActorRotation))
  (bind _velocityvector (Variables|Default|GetVelocityVector))
  (bind _returnvalue_2 (Math|Rotator|MakeRotfromX _velocityvector))
  (bind _returnvalue_3 (Math|Rotator|Delta(Rotator) _returnvalue _returnvalue_2))
  (if (Math|Float|InRange(Float) (.yaw _returnvalue_3) -2e+01 2e+01)
    (LocalVariables|SetDesiredAnimAsset "/Game/TransferDump/ControllerMain/Animations/InPlace/MOB1_Stand_Relaxed_to_Jog_F_IPC.MOB1_Stand_Relaxed_to_Jog_F_IPC")
    (elif (Math|Float|InRange(Float) (.yaw _returnvalue_3) -6e+01 -21.0)
      (LocalVariables|SetDesiredAnimAsset "/Game/TransferDump/ControllerMain/Animations/InPlace/MOB1_Stand_Relaxed_To_Jog_R45_Fwd_IPC.MOB1_Stand_Relaxed_To_Jog_R45_Fwd_IPC")
      (elif (Math|Float|InRange(Float) (.yaw _returnvalue_3) -1.1e+02 -61.0)
        (LocalVariables|SetDesiredAnimAsset "/Game/TransferDump/ControllerMain/Animations/InPlace/MOB1_Stand_Relaxed_To_Jog_R90_Fwd_IPC.MOB1_Stand_Relaxed_To_Jog_R90_Fwd_IPC")
        (elif (Math|Float|InRange(Float) (.yaw _returnvalue_3) -155.0 -1.1e+02)
          (LocalVariables|SetDesiredAnimAsset "/Game/TransferDump/ControllerMain/Animations/InPlace/MOB1_Stand_Relaxed_To_Jog_R135_Fwd_IPC.MOB1_Stand_Relaxed_To_Jog_R135_Fwd_IPC")
          (elif (Math|Float|InRange(Float) (.yaw _returnvalue_3) -1.8e+02 -155.0)
            (LocalVariables|SetDesiredAnimAsset "/Game/TransferDump/ControllerMain/Animations/InPlace/MOB1_Stand_Relaxed_To_Jog_R180_Fwd_IPC.MOB1_Stand_Relaxed_To_Jog_R180_Fwd_IPC")
            (elif (Math|Float|InRange(Float) (.yaw _returnvalue_3) 2e+01 6e+01)
              (LocalVariables|SetDesiredAnimAsset "/Game/TransferDump/ControllerMain/Animations/InPlace/MOB1_Stand_Relaxed_To_Jog_L45_Fwd_IPC.MOB1_Stand_Relaxed_To_Jog_L45_Fwd_IPC")
              (elif (Math|Float|InRange(Float) (.yaw _returnvalue_3) 6e+01 1.1e+02)
                (LocalVariables|SetDesiredAnimAsset "/Game/TransferDump/ControllerMain/Animations/InPlace/MOB1_Stand_Relaxed_To_Jog_L90_Fwd_IPC.MOB1_Stand_Relaxed_To_Jog_L90_Fwd_IPC")
                (elif (Math|Float|InRange(Float) (.yaw _returnvalue_3) 1.1e+02 155.0)
                  (LocalVariables|SetDesiredAnimAsset "/Game/TransferDump/ControllerMain/Animations/InPlace/MOB1_Stand_Relaxed_To_Jog_L135_Fwd_IPC.MOB1_Stand_Relaxed_To_Jog_L135_Fwd_IPC")
                  (elif (Math|Float|InRange(Float) (.yaw _returnvalue_3) 155.0 1.8e+02)
                    (LocalVariables|SetDesiredAnimAsset "/Game/TransferDump/ControllerMain/Animations/InPlace/MOB1_Stand_Relaxed_To_Jog_L180_Fwd_IPC.MOB1_Stand_Relaxed_To_Jog_L180_Fwd_IPC"))))))))))
  (return (LocalVariables|GetDesiredAnimAsset) (.yaw _returnvalue_3)))