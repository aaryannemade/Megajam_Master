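; Player pawn for a sacrifice mechanic, where each life leaves a Sacrifice_Light where it ends and teleports the player back to RespawnLocation.
; A looping LifeSpan timer ends each life automatically, while pressing E resets the timer and sacrifices immediately through the same logic.
; ReachedPoint clears the timer and adds text announcing arrival at the destination.
; Axis inputs drive yaw-relative movement and mouse look.
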(event Custom|Restart
  (Game|SpawnActorfromClass "/Game/Blueprints/Player/Sacrifice_Light.Sacrifice_Light_C" (Transformation|GetActorTransform) "AlwaysSpawn" 0 0)
  (Transformation|Teleport (Variables|Default|GetRespawnLocation) "0, 0, 0"))

(event Custom|ReachedPoint
  (Utilities|Time|ClearTimerbyFunctionName 0 "Restart")
  (bind _returnvalue (AddComponent|AddTextRenderComponent false (Math|Transform|MakeTransform "0.000000,-150.000000,75.000000" "0,180.000000, 0")))
  (Rendering|Components|TextRender|SetText _returnvalue (Utilities|Text|FormatText "You Have Reached The Destination")))

(event EventBeginPlay
  (Utilities|Time|SetTimerbyFunctionName 0 "Restart" (Variables|Default|GetLifeSpan) true))

(event Collision|EventActorBeginOverlap
  (params (OtherActor :type Actor%20Object%20Reference)))

(event EventTick
  (params (DeltaSeconds :type Float%20%28single-precision%29)))

(event Input|AxisEvents|InputAxisMoveForward
  (params (AxisValue :type Float%20%28single-precision%29))
  (Pawn|Input|AddMovementInput (Math|Vector|GetForwardVector (Math|Rotator|MakeRotator 0.0 0.0 (.yaw (Pawn|GetControlRotation :!class /Script/Engine.Pawn)))) AxisValue false))

(event Input|AxisEvents|InputAxisMoveRight
  (params (AxisValue :type Float%20%28single-precision%29))
  (Pawn|Input|AddMovementInput (Math|Vector|GetRightVector (Math|Rotator|MakeRotator 0.0 0.0 (.yaw (Pawn|GetControlRotation :!class /Script/Engine.Pawn)))) AxisValue false))

(event Input|AxisEvents|InputAxisMousePitch
  (params (AxisValue :type Float%20%28single-precision%29))
  (Pawn|Input|AddControllerPitchInput AxisValue))

(event Input|AxisEvents|InputAxisMouseYaw
  (params (AxisValue :type Float%20%28single-precision%29))
  (Pawn|Input|AddControllerYawInput AxisValue))

(event Input|KeyboardEvents|E
  (params (Key :type Key%20Structure))
  (:Pressed
    (Utilities|Time|ClearTimerbyFunctionName 0 "Restart")
    (Utilities|Time|SetTimerbyFunctionName 0 "Restart" (Variables|Default|GetLifeSpan) true)
    (Game|SpawnActorfromClass "/Game/Blueprints/Player/Sacrifice_Light.Sacrifice_Light_C" (Transformation|GetActorTransform) "AlwaysSpawn" 0 0)
    (Transformation|Teleport (Variables|Default|GetRespawnLocation) "0, 0, 0")))

(fn ConstructionScript)